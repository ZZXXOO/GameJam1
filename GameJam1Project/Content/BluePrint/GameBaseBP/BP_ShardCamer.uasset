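; BP_ShardCamer is a camera actor that becomes the first player's view and follows a gravity character.
; On BeginPlay it collects all BP_GravityCharacter actors, sets itself as player controller 0's view target and adds the UI_Camera widget to the viewport.
; Each Tick it snaps to the location of the first character found, without interpolation or sweep.
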(event `self.ReceiveBeginPlay`
  (bind _outactors (`GameplayStatics.GetAllActorsOfClass` "/DirGravity/Character/BP_GravityCharacter.BP_GravityCharacter_C"))
  (set `self.Characters` _outactors)
  (`PlayerController.SetViewTargetWithBlend` (`GameplayStatics.GetPlayerController` 0) self 0.0 "VTBlend_Linear" 0.0 false)
  (bind _returnvalue (`|CreateWidget` "/Game/ThirdPersonBP/Blueprints/UI_Camera.UI_Camera_C"))
  (`UserWidget.AddToViewport` _returnvalue 0))

(event `self.ReceiveTick`
  (params (DeltaSeconds :type "Float (single-precision)"))
  (`self.K2_SetActorLocation` (`self.K2_GetActorLocation` (`|GetArrayItem` (`self.Characters`)))))

(fn `UserConstructionScript`)