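; Game mode for a local two-player game that spawns and possesses both Paper2D characters at BeginPlay.
; It creates a second local player, places character two at the second PlayerStart or falls back to the first, and character one at the first.
; Character one receives a reference to character two, then a BP_ShardCamer actor is spawned, apparently as a shared camera.
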(event `self.ReceiveBeginPlay`
  (bind _output (`|GetArrayItem` (`self.PlayerStart`) 1))
  (`GameplayStatics.CreatePlayer` 1)
  (bind _outactors (`GameplayStatics.GetAllActorsOfClass` "/Script/Engine.PlayerStart"))
  (set `self.PlayerStart` _outactors)
  (`/Engine/EditorBlueprintResources/StandardMacros.IsValid` _output
    (:`Is Valid`
      (bind _returnvalue (`|SpawnActorFromClass` "/Game/Wmj/PaperCharacter2.PaperCharacter2_C" (`KismetMathLibrary.MakeTransform` (`self.K2_GetActorLocation` _output)) "Undefined" "OverrideRootScale" null null))
      (bind _output_get (set `self.PaperCharacter2BP` _returnvalue))
      (`Controller.Possess` (`GameplayStatics.GetPlayerController` 1) _output_get))
    (:`Is Not Valid`
      (bind _returnvalue_2 (`|SpawnActorFromClass` "/Game/Wmj/PaperCharacter2.PaperCharacter2_C" (`KismetMathLibrary.MakeTransform` (`self.K2_GetActorLocation` (`|GetArrayItem` (`self.PlayerStart`)))) "Undefined" "OverrideRootScale" null null))
      (bind _output_get_2 (set `self.PaperCharacter2BP` _returnvalue_2))
      (`Controller.Possess` (`GameplayStatics.GetPlayerController` 1) _output_get_2)))
  (bind _returnvalue_3 (`|SpawnActorFromClass` "/Game/ThirdPersonBP/Blueprints/PaperCharacter1.PaperCharacter1_C" (`KismetMathLibrary.MakeTransform` (`self.K2_GetActorLocation` (`|GetArrayItem` (`self.PlayerStart`)))) "Undefined" "OverrideRootScale" null null))
  (bind _output_get_3 (set `self.PaperCharacter1BP` _returnvalue_3))
  (`Controller.Possess` (`GameplayStatics.GetPlayerController` 0) _output_get_3)
  (set `/Game/ThirdPersonBP/Blueprints/PaperCharacter1.PaperCharacter2` (`self.PaperCharacter2BP`) _output_get_3)
  (`|SpawnActorFromClass` "/Game/BluePrint/GameBaseBP/BP_ShardCamer.BP_ShardCamer_C" (`KismetMathLibrary.MakeTransform` (0.0 0.0 0.0)) "AlwaysSpawn" "OverrideRootScale" null null))

(fn `UserConstructionScript`)